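; GA_Teleport is a Gameplay Ability that teleports the avatar pawn a short fixed distance along its facing direction.
; On activation it casts the avatar to Pawn and commits the ability, spawning a system effect at the departure point before teleporting with rotation unchanged.
; The ability ends whether or not the commit succeeds, but a failed Pawn cast stops execution without ending it.
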(event Ability|EventActivateAbility
  (bind _returnvalue (Ability|GetAvatarActorfromActorInfo))
  (bind _returnvalue_2 (Ability|GetAvatarActorfromActorInfo))
  (bind _returnvalue_3 (Transformation|GetActorRotation _returnvalue_2))
  (bind _returnvalue_4 (Transformation|GetActorRotation _returnvalue))
  (bind _aspawn (Utilities|Casting|CastToPawn (Ability|GetAvatarActorfromActorInfo)))
  (Variables|Default|SetAvatar%20Pawn _aspawn)
  (bind _returnvalue_5 (Ability|CommitAbility))
  (if _returnvalue_5
    (Niagara|SpawnSystematLocation 0 (+ (Transformation|GetActorLocation _returnvalue_2) (Math|Vector|GetForwardVector _returnvalue_3)) _returnvalue_3)
    (Transformation|Teleport (Variables|Default|GetAvatar%20Pawn) (+ (Transformation|GetActorLocation _returnvalue) (* (Math|Vector|GetForwardVector _returnvalue_4) 5e+02)) _returnvalue_4)
    (Ability|EndAbility)
    (else
      (Ability|EndAbility))))

(event Ability|EventOnEndAbility
  (params (bWasCancelled :type Boolean)))