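; Gameplay ability for a dash that boosts the player along their current motion.
; On activation it commits, then adds the avatar's velocity as a velocity-change impulse to player 0's character movement, roughly doubling speed when that player is the avatar.
; It spawns the NS_EnergyDash Niagara effect at the avatar, then immediately cancels itself.
; Disconnected nodes for normalized direction, friction and launching remain unused.
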(event Ability|EventActivateAbility
  (bind _returnvalue (Ability|GetAvatarActorfromActorInfo))
  (Ability|CommitAbility)
  (Physics|AddImpulse (Variables|/Script/Engine.Character|GetCharacterMovement (Game|GetPlayerCharacter 0)) (Transformation|GetVelocity _returnvalue) true)
  (Niagara|SpawnSystematLocation "/Game/Niagara/NS_EnergyDash.NS_EnergyDash" (Transformation|GetActorLocation _returnvalue) (Transformation|GetActorRotation _returnvalue))
  (Ability|CancelAbility))

(event Ability|EventOnEndAbility
  (params (bWasCancelled :type Boolean))
  (|CallParentFunction bWasCancelled) ; This node is disabled and will not be called.\nDrag off pins to build functionality.
)